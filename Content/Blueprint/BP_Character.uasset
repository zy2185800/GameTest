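; Player character Blueprint handling walk, run, jump and look input, with a limit on downward camera pitch.
; Run switches max walk speed instantly, and horizontal look input is also stored in OffSetZ.
; A looping timer started at BeginPlay picks idle, walk or run camera shake from velocity.
; Shoot only lights a SpotLight while held; the repeating gunfire sound logic is disconnected.
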(event EventBeginPlay
  (CallFunction|OpenCameraShake))

(event Input|ActionEvents|InputActionRun
  (params (Key :type Key%20Structure :default "None"))
  (bind _charactermovement (Variables|Character|GetCharacterMovement))
  ;[1 1 1] 奔跑(可优化细节 切换是速度插值)
  (:Pressed
    (Variables|/Script/Engine.CharacterMovementComponent|SetMaxWalkSpeed _charactermovement 6e+02))
  (:Released
    (Variables|/Script/Engine.CharacterMovementComponent|SetMaxWalkSpeed _charactermovement 2e+02)))

(event Input|ActionEvents|InputActionJump
  (params (Key :type Key%20Structure :default "None"))
  ;[1 1 1] 跳跃
  (:Pressed
    (Character|Jump))
  (:Released
    (Character|StopJumping)))

(event Input|AxisEvents|InputAxisMoveFoward
  (params (AxisValue :type Float%20%28single-precision%29))
  ;[1 1 1] 移动
  (Pawn|Input|AddMovementInput (Math|Vector|GetForwardVector (Transformation|GetWorldRotation (Variables|Collision|GetCapsuleComponent))) AxisValue false))

(event Input|AxisEvents|InputAxisMoveRight
  (params (AxisValue :type Float%20%28single-precision%29))
  ;[1 1 1] 移动
  (Pawn|Input|AddMovementInput (Math|Vector|GetRightVector (Transformation|GetWorldRotation (Variables|Collision|GetCapsuleComponent))) AxisValue false))

(event Input|AxisEvents|InputAxisLookUp
  (params (AxisValue :type Float%20%28single-precision%29))
  ;[1 1 1] 视角 以及向下视角的限制
  (if (> AxisValue 0.0)
    (if (> (.pitch (Transformation|GetWorldRotation (Variables|Default|GetCamera))) -7e+01)
      (Pawn|Input|AddControllerPitchInput AxisValue :!label _label))
    (else
      (goto _label))))

(event Input|AxisEvents|InputAxisLookRight
  (params (AxisValue :type Float%20%28single-precision%29))
  ;[1 1 1] 视角 以及向下视角的限制
  (Pawn|Input|AddControllerYawInput AxisValue)
  (Variables|Default|SetOffSet_Z AxisValue))

(event Input|ActionEvents|InputActionShoot
  (params (Key :type Key%20Structure :default "None"))
  (bind _spotlight (Variables|Default|GetSpotLight))
  (:Pressed
    (Rendering|Components|Light|SetIntensity _spotlight 8e+03))
  (:Released
    (Rendering|Components|Light|SetIntensity _spotlight 0.0)))

(event Custom|OpenCameraShake
  ;[1 1 1] 镜头晃动
  (Utilities|Time|SetTimerbyEvent (delegate Custom|人物正常状态模拟) 0.4 true))

(event Custom|人物正常状态模拟
  (bind _returnvalue (Transformation|GetVelocity))
  (bind _returnvalue_2 (Game|GetPlayerCameraManager 0))
  (bind _returnvalue_3 (Math|Vector|VectorLength _returnvalue))
  ;[1 1 1] 镜头晃动
  (if (> _returnvalue_3 3.1e+02)
    (Class|PlayerCameraManager|PlayCameraShake _returnvalue_2 "/Game/Blueprint/镜头晃动/RunShake.RunShake_C" 1.0 "CameraLocal" "0, 0, 0")
    (elif (> _returnvalue_3 1e+01)
      (Class|PlayerCameraManager|PlayCameraShake _returnvalue_2 "/Game/Blueprint/镜头晃动/WalkShake.WalkShake_C" 1.0 "CameraLocal" "0, 0, 0")
      (else
        (Class|PlayerCameraManager|PlayCameraShake _returnvalue_2 "/Game/Blueprint/镜头晃动/IdleShake.IdleShake_C" 1.0 "CameraLocal" "0, 0, 0")))))

(fn ConstructionScript)